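; BP_MonsterSphereClass is a spawner volume that populates an area with AI monsters when a level begins.
; On BeginPlay it spawns up to MaxSpawnNum monsters at random reachable points within the sphere via a delayed loop, then destroys itself; on a loaded game it destroys itself immediately.
; Each spawn registers in the FogGamemode's AllSpawnMonster list, and a separate event spawns a given monster class on demand.
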(event Custom|Event_SpawnMonster
  (params (SpawnMonsterClass :type Pawn%20Class%20Reference))
  ;[1 1 1] 生成怪物
  (bind _returnvalue (AI|SpawnAIFromClass SpawnMonsterClass 0 (.RandomLocation (AI|Navigation|GetRandomReachablePointinRadius (Transformation|GetWorldLocation (Variables|Default|GetSphere)) (Variables|SpawnSet|GetSpawnSphereRadius) 0 0)) "0, 0, 0" false 0))
  (bind _asbp_monster_class (Utilities|Casting|CastToBP_MonsterClass _returnvalue))
  (Utilities|Array|Add (Variables|/Game/BP/BP_FogGamemode.BP_FogGamemode_C|GetAllSpawnMonster (Variables|Default|GetBP%20Fog%20Gamemode)) _asbp_monster_class))

(event EventBeginPlay
  ;[1 1 1] 初始化生成怪物
  (Variables|Default|SetBP%20Fog%20Gamemode (.AsBP%20Fog%20Gamemode (Utilities|Casting|CastToBP_FogGamemode (Game|GetGameMode))))
  (if (Variables|/Game/BP/BP_FogGameInstance.BP_FogGameInstance_C|GetIsLoad (.AsBP%20Fog%20Game%20Instance (Utilities|Casting|CastToBP_FogGameInstance (Game|GetGameInstance))))
    (Actor|DestroyActor)
    (else
      (Utilities|DelayforLoop 1 (Variables|SpawnSet|GetMaxSpawnNum) (Variables|SpawnSet|GetSpawnDuration)
        (:Loop
          (bind _returnvalue (AI|SpawnAIFromClass (Variables|SpawnSet|GetSpawnMonsterClass) 0 (.RandomLocation (AI|Navigation|GetRandomReachablePointinRadius (Transformation|GetWorldLocation (Variables|Default|GetSphere)) (Variables|SpawnSet|GetSpawnSphereRadius) 0 0)) "0, 0, 0" true 0))
          (bind _asbp_monster_class (Utilities|Casting|CastToBP_MonsterClass _returnvalue))
          (Utilities|Array|Add (Variables|/Game/BP/BP_FogGamemode.BP_FogGamemode_C|GetAllSpawnMonster (Variables|Default|GetBP%20Fog%20Gamemode)) _asbp_monster_class))
        (:LoopEnd
          (Actor|DestroyActor))))))

(fn ConstructionScript
  (Components|Sphere|SetSphereRadius (Variables|Default|GetSphere) (Variables|SpawnSet|GetSpawnSphereRadius) true))