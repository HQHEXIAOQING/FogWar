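; Game mode for a fog-themed game that manages the main, pause and end-screen widgets, loading and the win check.
; On BeginPlay it gathers save lights, and when the game instance flags a load it restores player location, spawned monsters and saved lights by ID.
; Monsters passed to the estimate event leave the tracked list, and an empty list triggers the success screen.
; Pausing works by setting global time dilation to zero.
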(event Custom|Event_Estimate
  (params (Monster :type BP%20Monster%20Class%20Object%20Reference))
  (bind _allspawnmonster (Variables|Default|GetAllSpawnMonster))
  ;[1 1 1] 判断游戏是否胜利
  (Utilities|Array|RemoveItem _allspawnmonster Monster)
  (if (not (> (Utilities|Array|Length _allspawnmonster) 0))
    (CallFunction|EventSucceed true)))

(event Custom|Event_Succeed
  (params (GameSucceed :type Boolean))
  (bind _umg_gameend (Variables|UMGSet|GetUMG_GameEnd))
  ;[1 1 1] 结束事件
  (Pawn|Components|CharacterMovement|SetMovementMode (Variables|/Script/Engine.Character|GetCharacterMovement (Variables|Default|GetPlayer)) "MOVE_None" 0)
  (Input|SetInputModeUIOnly (Game|GetPlayerController 0) 0 "DoNotLock" false)
  (Widget|RemovefromParent (Variables|UMGSet|GetUMG_GameMain))
  (UserInterface|Viewport|AddtoViewport _umg_gameend 0)
  (Default|EventGameEnd _umg_gameend GameSucceed))

(event Custom|Event_SaveGameBegin
  (bind _bp_fog_game_instance (Variables|Default|GetBP%20Fog%20Game%20Instance))
  (bind _lastsave_game (Variables|/Game/BP/BP_FogGameInstance.BP_FogGameInstance_C|GetLastSave%20Game _bp_fog_game_instance))
  (bind (_savegamename _playerlocation _monsterlocation _monsterclass _savelightid) (Utilities|Struct|BreakDS_HQSaveGame _lastsave_game))
  ;[1 1 1] 加载游戏
  (Utilities|Array|Clear (Variables|Default|GetAllSpawnMonster))
  (Transformation|SetActorLocation (Variables|Default|GetPlayer) _playerlocation false false)
  (Utilities|FlowControl|Delay 0.2)
  (for (_array_element _array_index) _monsterlocation
    (bind _returnvalue (Game|SpawnActorfromClass (Utilities|Array|Get(acopy) _monsterclass _array_index) (Math|Transform|MakeTransform _array_element "0, 0, 0" "1.000000,1.000000,1.000000") "Undefined" "MultiplyWithRoot" 0 0))
    (bind _asbp_monster_class (Utilities|Casting|CastToBP_MonsterClass _returnvalue))
    (Utilities|IsValid _asbp_monster_class
      (:Is%20Valid
        (Default|EventRandomMove _asbp_monster_class)
        (Utilities|Array|Add (Variables|Default|GetAllSpawnMonster) _asbp_monster_class))))
  (for _array_element_2 _savelightid
    (for _array_element_3 (Variables|Default|GetAllSaveLight)
      (if (== (Variables|/Game/BP/LightClass/BP_LightFogClass.BP_LightFogClass_C|GetLightSaveID _array_element_3) _array_element_2)
        (Default|EventSaveGame _array_element_3)
        (Development|PrintString (Utilities|GetDisplayName _array_element_3))))))

(event EventBeginPlay
  ;[1 1 1] 事件初始化
  (bind _outactors (Actor|GetAllActorsOfClass "/Game/BP/LightClass/BP_LightFogClass.BP_LightFogClass_C"))
  (Variables|Default|SetAllSaveLight _outactors)
  (Variables|Default|SetBP%20Fog%20Game%20Instance (.AsBP%20Fog%20Game%20Instance (Utilities|Casting|CastToBP_FogGameInstance (Game|GetGameInstance))))
  (bind _returnvalue (UserInterface|CreateWidget "/Game/UMG/UMG_Game/UMG_GameStop.UMG_GameStop_C"))
  (Variables|UMGSet|SetUMG_GameStop _returnvalue)
  (bind _returnvalue_2 (UserInterface|CreateWidget "/Game/UMG/UMG_Game/UMG_GameMain.UMG_GameMain_C"))
  (bind _output_get (Variables|UMGSet|SetUMG_GameMain _returnvalue_2))
  (UserInterface|Viewport|AddtoViewport _output_get 0)
  (bind _returnvalue_3 (Game|ConstructObjectfromClass "/Game/UMG/UMG_Game/UMG_GameEnd.UMG_GameEnd_C"))
  (Variables|UMGSet|SetUMG_GameEnd _returnvalue_3)
  (bind _asbp_player_class (Utilities|Casting|CastToBP_PlayerClass (Game|Player|GetPlayerPawn 0)))
  (Variables|Default|SetPlayer _asbp_player_class)
  (Input|SetInputModeGameandUI (Game|GetPlayerController 0) 0 "DoNotLock" true false)
  (if (Variables|/Game/BP/BP_FogGameInstance.BP_FogGameInstance_C|GetIsLoad (Variables|Default|GetBP%20Fog%20Game%20Instance))
    (CallFunction|EventSaveGameBegin)))

(event Custom|Event_RemoveGameStop
  ;[1 1 1] 显示和移除暂停界面
  (Utilities|Time|SetGlobalTimeDilation 1.0)
  (Widget|RemovefromParent (Variables|UMGSet|GetUMG_GameStop)))

(event Custom|Event_OpenGameStop
  ;[1 1 1] 显示和移除暂停界面
  (Utilities|Time|SetGlobalTimeDilation 0.0)
  (UserInterface|Viewport|AddtoViewport (Variables|UMGSet|GetUMG_GameStop) 0))

(fn ConstructionScript)