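; Fog light checkpoint actor that auto-saves the game the first time the player walks into its trigger sphere.
; The construction script sizes the trigger from SphereRadius, and BeginPlay hides the screen-space text widget and gives the Sphere a dynamic light material.
; Overlap stores the player and runs the save event, which sets the material's Switch parameter, destroys the trigger and marks IsSave, alongside calling AutoSaveGame.
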(event OnComponentBeginOverlap(Sphere1)
  (params (OverlappedComponent :type Primitive%20Component%20Object%20Reference) (OtherActor :type Actor%20Object%20Reference) (OtherComp :type Primitive%20Component%20Object%20Reference) (OtherBodyIndex :type Integer) (bFromSweep :type Boolean) (SweepResult :type Hit%20Result%20Structure%20%28by%20ref%29))
  ;[1 1 1] 存档游戏
  (bind _asbp_player_class (Utilities|Casting|CastToBP_PlayerClass OtherActor))
  (Utilities|FlowControl|DoOnce false
    (:Completed
      (Variables|Default|SetPlayer _asbp_player_class)
      (CallFunction|EventSaveGame)
      (Utilities|AutoSaveGame true))))

(event Custom|Event_SaveGame
  ;[1 1 1] 存档完成设置
  (Rendering|Material|SetScalarParameterValue (Variables|Default|GetDM_Light) "Switch" 1.0 :!class /Script/Engine.MaterialInstanceDynamic)
  (Components|DestroyComponent (Variables|Default|GetSphere1))
  (Variables|Default|SetIsSave？ true))

(event EventBeginPlay
  (bind _showtext (Variables|Default|GetShowText))
  ;[1 1 1] 初始化设置
  (Class|WidgetComponent|SetWidgetSpace _showtext "Screen")
  (Rendering|SetVisibility _showtext false false)
  (bind _returnvalue (Rendering|Material|CreateDynamicMaterialInstance "/Game/BP/LightClass/Assets_LightClass/Mat_Light_01.Mat_Light_01" "None" "None" :!class /Script/Engine.KismetMaterialLibrary))
  (Variables|Default|SetDM_Light _returnvalue)
  (Rendering|Material|SetMaterial (Variables|Default|GetSphere) 0 (Variables|Default|GetDM_Light))
  (Variables|Default|SetBP%20Fog%20Gamemode (.AsBP%20Fog%20Gamemode (Utilities|Casting|CastToBP_FogGamemode (Game|GetGameMode)))))

(fn ConstructionScript
  (Components|Sphere|SetSphereRadius (Variables|Default|GetSphere1) (Variables|Default|GetSphereRadius) true))