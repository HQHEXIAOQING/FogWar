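; Base monster character for the fog game mode that detects, chases and melee-attacks players.
; A radius-configurable sphere sets the target, switching between random navmesh moves and AIMoveTo pursuit into a repeating attack montage whose notify sphere-traces from the staff to apply damage.
; It starts hidden, with EventShowHP toggling mesh, staff, HP widget and minimap tag together.
; At zero HP it notifies the game mode, ragdolls and is destroyed after a delay.
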(event OnComponentBeginOverlap(Sphere)
  (params (OverlappedComponent :type Primitive%20Component%20Object%20Reference) (OtherActor :type Actor%20Object%20Reference) (OtherComp :type Primitive%20Component%20Object%20Reference) (OtherBodyIndex :type Integer) (bFromSweep :type Boolean) (SweepResult :type Hit%20Result%20Structure%20%28by%20ref%29))
  ;[1 1 1] 碰撞检测玩家是否在攻击范围内
  (if (not (Variables|Default|GetIsDie))
    (bind _asbp_player_class (Utilities|Casting|CastToBP_PlayerClass OtherActor))
    (Variables|Default|SetPlayer _asbp_player_class)
    (CallFunction|EventFindPlayer)))

(event OnComponentEndOverlap(Sphere)
  (params (OverlappedComponent :type Primitive%20Component%20Object%20Reference) (OtherActor :type Actor%20Object%20Reference) (OtherComp :type Primitive%20Component%20Object%20Reference) (OtherBodyIndex :type Integer))
  ;[1 1 1] 碰撞检测玩家是否在攻击范围内
  (if (not (Variables|Default|GetIsDie))
    (Utilities|Casting|CastToBP_PlayerClass OtherActor)
    (Variables|Default|SetPlayer 0)
    (CallFunction|EventRandomMove)))

(event Custom|Event_RandomMove
  ;[1 1 1] 随机移动
  (if (not (Variables|Default|GetIsDie))
    (bind _randomlocation (Class|NavigationSystemV1|GetRandomLocationinNavigableRadius (Transformation|GetActorLocation) (Variables|MonsterSet|GetFindRadius) 0 0))
    (AI|AIMoveTo self _randomlocation 0 5.0 false)))

(event Custom|Event_FindPlayer
  ;[1 1 1] 查找玩家并追逐
  (if (not (Variables|Default|GetIsDie))
    (bind _player (Variables|Default|GetPlayer)
      (:then
        (if (not (Variables|/Game/BP/BP_FogChr/BP_Player/BP_PlayerClass.BP_PlayerClass_C|GetIsDie _player))
          (AI|AIMoveTo self "0, 0, 0" _player 1.5e+02 false
            (:OnSuccess
              (CallFunction|EventAttack)))))
      (:else
        (CallFunction|EventRandomMove)))))

(event Custom|Event_Attack
  (bind _staff01sm (Variables|Default|GetStaff01SM))
  (bind _returnvalue (Transformation|GetWorldLocation _staff01sm))
  ;[1 1 1] 攻击的逻辑
  (bind _player (Variables|Default|GetPlayer :!label _label)
    (:then
      (if (not (Variables|/Game/BP/BP_FogChr/BP_Player/BP_PlayerClass.BP_PlayerClass_C|GetIsDie _player))
        (if (<= (Transformation|GetDistanceTo self _player) 3e+02)
          (bind _notifyname (Animation|Montage|PlayMontage (Variables|Character|GetMesh) "/Game/Assets/SKMesh/Montage/MonsterMontage/MTQ_Attack_Monster01.MTQ_Attack_Monster01")
            (:OnCompleted
              (goto _label))
            (:OnNotifyBegin
              (switch name _notifyname
                (:Attack
                  (bind _outhit (Collision|SphereTraceForObjects _returnvalue _returnvalue 2e+02 (Utilities|Array|MakeArray "ObjectTypeQuery7") false 0 "None"))
                  (bind _asbp_player_class (Utilities|Casting|CastToBP_PlayerClass (.HitActor (Collision|BreakHitResult _outhit))))
                  (Game|Damage|ApplyDamage _asbp_player_class (.atk (Variables|MonsterSet|GetMonsterData)) 0 self)))))
          (else
            (CallFunction|EventFindPlayer)))))
    (:else
      (CallFunction|EventRandomMove))))

(event Custom|Event_ShowHP
  (params (IsShow :type Boolean))
  (bind _bpc_minimap (Variables|Default|GetBPC_MiniMap))
  ;[1 1 1] 设置血条和图标显示
  (if (not (Variables|Default|GetIsDie))
    (Rendering|SetVisibility (Variables|Character|GetMesh) IsShow false)
    (if IsShow
      (Default|EventAddTagUMG _bpc_minimap)
      (else
        (Default|EventRemoveTagTex _bpc_minimap)))))

(event EventBeginPlay
  (bind _widget (Variables|Default|GetWidget))
  ;[1 1 1] 初始化设置
  (Variables|Default|SetFogGamemode (.AsBP%20Fog%20Gamemode (Utilities|Casting|CastToBP_FogGamemode (Game|GetGameMode))))
  (Variables|/Script/Engine.CharacterMovementComponent|SetMaxWalkSpeed (Variables|Character|GetCharacterMovement) 5e+02)
  (Class|WidgetComponent|SetWidgetSpace _widget "Screen")
  (bind _output_get (Variables|Default|SetUMGMonster (.AsBPU%20Monster%20HP (Utilities|Casting|CastToBPU_MonsterHP (UserInterface|GetWidget _widget)))))
  (Variables|/Game/BP/BP_FogChr/BP_Monster/BPU_MonsterHP.BPU_MonsterHP_C|SetOwerMonster _output_get self)
  (CallFunction|EventShowHP false)
  (Variables|Default|SetIsDie false)
  (Utilities|FlowControl|Delay (Math|Random|RandomFloatinRange 0.5 2.0))
  (Variables|Default|GetPlayer
    (:then)
    (:else
      (CallFunction|EventRandomMove))))

(event Game|Damage|EventAnyDamage
  (params (Damage :type Float%20%28single-precision%29) (DamageType :type Damage%20Type%20Object%20Reference) (InstigatedBy :type Controller%20Object%20Reference) (DamageCauser :type Actor%20Object%20Reference))
  (bind _monsterdata (Variables|MonsterSet|GetMonsterData))
  (bind _monsterdata_2 (Variables|MonsterSet|GetMonsterData))
  (bind _returnvalue (- (.hp _monsterdata) Damage))
  ;[1 1 1] 受到攻击事件
  (if (> _returnvalue 0.0)
    (Utilities|Struct|SetmembersinDS_MonsterData _monsterdata_2 _returnvalue)
    (else
      (Utilities|Struct|SetmembersinDS_MonsterData _monsterdata_2 0.0)
      (Variables|Default|SetIsDie true)
      (Default|EventEstimate (Variables|Default|GetFogGamemode) self)
      (Physics|SetSimulatePhysics (Variables|Character|GetMesh) true)
      (Collision|SetCollisionEnabled (Variables|Default|GetCapsuleComponent) "NoCollision")
      (Utilities|FlowControl|Delay 2.0)
      (Default|EventRemoveTagTex (Variables|Default|GetBPC_MiniMap))
      (Actor|DestroyActor))))

(fn ConstructionScript
  (|CallParentFunction)
  (Components|Sphere|SetSphereRadius (Variables|Default|GetSphere) (Variables|MonsterSet|GetCollisionRadius) true))