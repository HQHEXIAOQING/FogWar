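; BP_BulletClass is a projectile actor that deals damage to monsters on behalf of the player who fired it.
; Event_Attack stores the shooter and attack value, launches the physics Mesh with an impulse along the given direction, and destroys the bullet after a short delay.
; On a Mesh hit, a BP_MonsterClass target takes damage once through a DoOnce before the bullet is destroyed, while any other hit just destroys it.
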(event OnComponentHit(Mesh)
  (params (HitComponent :type Primitive%20Component%20Object%20Reference) (OtherActor :type Actor%20Object%20Reference) (OtherComp :type Primitive%20Component%20Object%20Reference) (NormalImpulse :type Vector :default "0, 0, 0") (Hit :type Hit%20Result%20Structure%20%28by%20ref%29))
  ;[1 1 1] 碰撞检测
  (bind _asbp_monster_class (Utilities|Casting|CastToBP_MonsterClass OtherActor)
    (:then
      (Utilities|FlowControl|DoOnce false
        (:Completed
          (Game|Damage|ApplyDamage _asbp_monster_class (Variables|Default|GetATK) 0 (Variables|Default|GetPlayer))
          (Actor|DestroyActor))))
    (:CastFailed
      (Actor|DestroyActor))))

(event Custom|Event_Attack
  (params (Player :type BP%20Player%20Class%20Object%20Reference) (ATK :type Float%20%28double-precision%29) (Direction :type Vector))
  ;[1 1 1] 事件初始化攻击。
  (Variables|Default|SetPlayer Player)
  (Variables|Default|SetATK ATK)
  (Physics|AddImpulse (Variables|Default|GetMesh) (* Direction (Variables|BulletData|GetBulletSpeed)) "None" false)
  (Utilities|FlowControl|Delay 2.0)
  (Actor|DestroyActor))

(fn ConstructionScript)