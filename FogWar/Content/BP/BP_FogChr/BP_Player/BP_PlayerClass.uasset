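; Player character class with world-axis movement, hold-to-sprint and a mouse-aimed projectile attack.
; Attacking plays a gated montage and traces from the cursor for a monster or ground point; the Attack notify turns the player toward it and spawns a bullet carrying PlayerData's ATK.
; Damage drains HP; at zero the mesh ragdolls and the game mode is told of failure.
; Look and camera-switch inputs are empty stubs.
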(event Custom|Event_Attack
  ;[1 1 1] 普通攻击/上
  (bind _returnvalue (Game|SpawnActorfromClass "/Game/BP/BP_FogChr/BP_Player/BP_BulletChild/BP_Bullet01.BP_Bullet01_C" (Math|Transform|MakeTransform (Transformation|GetWorldLocation (Variables|Default|GetBulletArrow)) "0, 0, 0" "1.000000,1.000000,1.000000") "Undefined" "MultiplyWithRoot" 0 0))
  (bind _asbp_bullet_class (Utilities|Casting|CastToBP_BulletClass _returnvalue))
  (Utilities|IsValid _asbp_bullet_class
    (:Is%20Valid
      (Default|EventAttack _asbp_bullet_class self (.atk (Variables|PlayerDataSet|GetPlayerData)) (Variables|BulletSet|GetBulletDirection)))))

(event Input|EnhancedActionEvents|EnhancedInputActionIA_move
  (params (ActionValue :type Vector%202D%20Structure) (ElapsedSeconds :type Float%20%28double-precision%29) (TriggeredSeconds :type Float%20%28double-precision%29) (InputAction :type Input%20Action%20Object%20Reference :default "/Game/KNQ/IA/IA_move.IA_move"))
  ;[1 1 1] 移动输入设置
  (Pawn|Input|AddMovementInput (Math|Vector|MakeVector (.x ActionValue) (.y ActionValue) 0.0) 1.0 false))

(event Input|EnhancedActionEvents|EnhancedInputActionIA_look
  (params (ActionValue :type Vector%202D%20Structure) (ElapsedSeconds :type Float%20%28double-precision%29) (TriggeredSeconds :type Float%20%28double-precision%29) (InputAction :type Input%20Action%20Object%20Reference :default "/Game/KNQ/IA/IA_look.IA_look"))
  ;[1 0 0] 这个暂时觉得不需要，先不要做旋转输入吧
)

(event Input|EnhancedActionEvents|EnhancedInputActionIA_SetArm
  (params (ActionValue :type Boolean) (ElapsedSeconds :type Float%20%28double-precision%29) (TriggeredSeconds :type Float%20%28double-precision%29) (InputAction :type Input%20Action%20Object%20Reference :default "/Game/KNQ/IA/IA_SetArm.IA_SetArm"))
  ;[1 1 1] 添加视角切换
)

(event Input|EnhancedActionEvents|EnhancedInputActionIA_highspeed
  (params (ActionValue :type Boolean) (ElapsedSeconds :type Float%20%28double-precision%29) (TriggeredSeconds :type Float%20%28double-precision%29) (InputAction :type Input%20Action%20Object%20Reference :default "/Game/KNQ/IA/IA_highspeed.IA_highspeed"))
  (bind _charactermovement (Variables|Character|GetCharacterMovement))
  ;[1 1 1] 切换疾跑（还需要耐力值）
  (:Started
    (Variables|/Script/Engine.CharacterMovementComponent|SetMaxWalkSpeed _charactermovement 6e+02))
  (:Completed
    (Variables|/Script/Engine.CharacterMovementComponent|SetMaxWalkSpeed _charactermovement 4.5e+02)))

(event Input|EnhancedActionEvents|EnhancedInputActionIA_Nrm_attack
  (params (ActionValue :type Boolean) (ElapsedSeconds :type Float%20%28double-precision%29) (TriggeredSeconds :type Float%20%28double-precision%29) (InputAction :type Input%20Action%20Object%20Reference :default "/Game/KNQ/IA/IA_Nrm_attack.IA_Nrm_attack"))
  ;[1 1 1] 普通攻击/上
  (:Started
    (Utilities|FlowControl|Gate false :!label _label
      (:Exit
        (bind _notifyname (Animation|Montage|PlayMontage (Variables|Character|GetMesh) "/Game/Assets/SKMesh/Montage/PlayerMontage/MTQ_Attack_Player01.MTQ_Attack_Player01" 3.0)
          (:then
            (CallFunction|FunDetectionAttack)
            (goto _label Close))
          (:OnCompleted
            (goto _label Open))
          (:OnNotifyBegin
            (switch name _notifyname
              (:Attack
                (CallFunction|FunGetBulletSpeed)
                (CallFunction|EventAttack)))))))))

(event EventBeginPlay
  ;[1 1 1] 初始化设置
  (Variables|BaseClassSet|SetBP%20Fog%20Gamemode (.AsBP%20Fog%20Gamemode (Utilities|Casting|CastToBP_FogGamemode (Game|GetGameMode))))
  (bind _output_get (Variables|BaseClassSet|SetBP%20Fog%20Controller (.AsBP%20Fog%20Controller (Utilities|Casting|CastToBP_FogController (Game|GetPlayerController 0)))))
  (Input|AddMappingContext (PlayerController|LocalPlayerSubsystems|GetEnhancedInputLocalPlayerSubsystem _output_get) "/Game/KNQ/IA/IMC_Magical.IMC_Magical" 0 "(bIgnoreAllPressedKeysUntilRelease=True,bForceImmediately=False,bNotifyUserSettings=False)")
  (Variables|/Script/Engine.CharacterMovementComponent|SetMaxWalkSpeed (Variables|Character|GetCharacterMovement) 4.5e+02)
  (Variables|Default|SetIsDie false))

(event Game|Damage|EventAnyDamage
  (params (Damage :type Float%20%28single-precision%29) (DamageType :type Damage%20Type%20Object%20Reference) (InstigatedBy :type Controller%20Object%20Reference) (DamageCauser :type Actor%20Object%20Reference))
  (bind _playerdata (Variables|PlayerDataSet|GetPlayerData))
  (bind _playerdata_2 (Variables|PlayerDataSet|GetPlayerData))
  (bind _returnvalue (- (.hp _playerdata) Damage))
  ;[1 1 1] 伤害死亡事件判断
  (if (not (Variables|Default|GetIsDie))
    (if (> _returnvalue 0.0)
      (Utilities|Struct|SetmembersinDS_PlayerData _playerdata_2 _returnvalue)
      (else
        (Utilities|Struct|SetmembersinDS_PlayerData _playerdata_2 0.0)
        (Variables|Default|SetIsDie true)
        (Physics|SetSimulatePhysics (Variables|Character|GetMesh) true)
        (Default|EventSucceed (Variables|BaseClassSet|GetBP%20Fog%20Gamemode) false)))))

(fn ConstructionScript
  (|CallParentFunction))

(fn FunDetectionAttack
  (bind _bp_fog_controller (Variables|BaseClassSet|GetBP%20Fog%20Controller))
  (bind (_worldlocation _worlddirection) (Game|Player|ConvertMouseLocationToWorldSpace _bp_fog_controller))
  (Utilities|FlowControl|Sequence
    (:then_0
      (bind _outhit (Collision|LineTraceForObjects _worldlocation (+ _worldlocation (* _worlddirection 7e+03)) (Utilities|Array|MakeArray "ObjectTypeQuery3" "ObjectTypeQuery1") false 0 "None"))
      (if (.bBlockingHit (Collision|BreakHitResult _outhit))
        (bind _asbp_monster_class (Utilities|Casting|CastToBP_MonsterClass (.HitActor (Collision|BreakHitResult _outhit)))
          (:then
            (Variables|BulletSet|SetClickMonster _asbp_monster_class))
          (:CastFailed
            (Variables|BulletSet|SetLocation (.Location (Collision|BreakHitResult _outhit)) :!label _label)
            (Variables|BulletSet|SetClickMonster 0)))
        (else
          (goto _label))))
    (:then_1
      (return))))

(fn FunGetBulletSpeed
  (bind _returnvalue (Transformation|GetActorLocation))
  (bind _location (Variables|BulletSet|GetLocation))
  (bind _returnvalue_2 (Math|Rotator|FindLookatRotation _returnvalue (Math|Vector|MakeVector (.x _location) (.y _location) 1e+02)))
  (bind _clickmonster (Variables|BulletSet|GetClickMonster)
    (:then
      (Variables|BulletSet|SetBulletDirection (Math|Vector|GetForwardVector (Math|Rotator|FindLookatRotation (Transformation|GetActorLocation) (Transformation|GetActorLocation _clickmonster))))
      (Transformation|SetActorRotation (Math|Rotator|FindLookatRotation (Transformation|GetActorLocation) (Transformation|GetActorLocation _clickmonster)))
      (return))
    (:else
      (Variables|BulletSet|SetBulletDirection (Math|Vector|GetForwardVector _returnvalue_2))
      (Transformation|SetActorRotation _returnvalue_2)
      (return))))