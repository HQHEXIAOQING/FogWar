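; Player follow-camera actor with a spring arm that can switch between two zoom distances.
; Each Tick eases the actor toward the Player's location at a speed scaled by max walk speed and CameraSpeed, and inversely by arm length.
; A FlipFlop event toggles the target arm length between far and near, and Tick smoothly interpolates the spring arm toward it.
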(event Custom|Event_SetArmLength
  ;[1 1 1] 设置弹簧臂的长度
  (Utilities|FlowControl|FlipFlop
    (:A
      (Variables|Default|SetSwitchArmLength 2.5e+03))
    (:B
      (Variables|Default|SetSwitchArmLength 1.5e+03))))

(event EventTick
  (params (DeltaSeconds :type Float%20%28single-precision%29))
  ;[1 1 1] Tick设置摄像机的位置
  (bind _player (Variables|Default|GetPlayer)
    (:then
      (Transformation|SetActorLocation (.ReturnValue (CallFunction|FunGetCameraLocation _player)) false false)
      (Variables|/Script/Engine.SpringArmComponent|SetTargetArmLength (Variables|Default|GetSpringArm) (.ArmLength (CallFunction|FunGetCameraLocation _player))))
    (:else)))

(fn ConstructionScript)

(fn FunGetCameraLocation
  (params (Player :type Character%20Object%20Reference))
  (bind _returnvalue (Utilities|Time|GetWorldDeltaSeconds))
  (bind _springarm (Variables|Default|GetSpringArm))
  (bind _switcharmlength (Variables|Default|GetSwitchArmLength))
  (bind _targetarmlength (Variables|/Script/Engine.SpringArmComponent|GetTargetArmLength _springarm))
  (return (Math|Interpolation|VInterpTo (Transformation|GetActorLocation) (Transformation|GetActorLocation Player) _returnvalue (/ (Variables|/Script/Engine.CharacterMovementComponent|GetMaxWalkSpeed (Variables|/Script/Engine.Character|GetCharacterMovement Player)) (/ (Variables|/Script/Engine.SpringArmComponent|GetTargetArmLength (Variables|Default|GetSpringArm)) (Variables|Default|GetCameraSpeed)))) (select (Math|Float|NearlyEqual(Float) _targetarmlength _switcharmlength 0.2) _targetarmlength (Math|Interpolation|FInterpTo _targetarmlength _switcharmlength _returnvalue 1.0))))