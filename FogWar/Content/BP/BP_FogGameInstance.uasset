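; Game instance that manages persistence of player settings and game progress through two save-game classes.
; On first start it async-loads or creates the settings save once, then hands the settings to the main start UMG widget.
; Game progress is read from the "Auto" slot, or a new save object is created if none exists.
; Saving writes settings back, or game data to a caller-named slot, creating that save when missing.
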(event Custom|Event_Begin
  (params (UMG_MainStart :type UMG%20Start%20Main%20Object%20Reference))
  ;[1 1 1] 设置数据初始化设置
  (Variables|SaveSet|SetUMG_MainStart UMG_MainStart)
  (Utilities|FlowControl|DoOnce false
    (:Completed
      (Variables|SaveSet|SetIsSaveGameSetOK false)
      (bind _returnvalue (SaveGame|DoesSaveGameExist (Variables|SaveSet|GetSetSlot)))
      (if _returnvalue
        (bind _savegame (|AsyncLoadGamefromSlot (Variables|SaveSet|GetSetSlot))
          (:Completed
            (Variables|SaveSet|SetBP_SetSaveGame (.AsBP%20Fog%20Save%20Set (Utilities|Casting|CastToBP_FogSaveSet _savegame)))
            (Variables|SaveSet|SetIsSaveGameSetOK true)))
        (else
          (bind _returnvalue_2 (SaveGame|CreateSaveGameObject "/Game/BP/SaveGame/BP_FogSaveSet.BP_FogSaveSet_C"))
          (bind _output_get (Variables|SaveSet|SetBP_SetSaveGame _returnvalue_2))
          (|AsyncSaveGametoSlot self _output_get (Variables|SaveSet|GetSetSlot)
            (:Completed
              (Variables|SaveSet|SetIsSaveGameSetOK true)))))
      (bind _output_get_2 (Variables|SaveSet|SetLastDS_SaveSet (Variables|/Game/BP/SaveGame/BP_FogSaveSet.BP_FogSaveSet_C|GetDS_SaveSet (Variables|SaveSet|GetBP_SetSaveGame))))
      (Default|EventBeginSet (Variables|SaveSet|GetUMG_MainStart) _output_get_2))))

(event Custom|Event_SaveSet
  (bind _bp_setsavegame (Variables|SaveSet|GetBP_SetSaveGame))
  ;[1 1 1] 保存设置内容
  (Variables|/Game/BP/SaveGame/BP_FogSaveSet.BP_FogSaveSet_C|SetDS_SaveSet _bp_setsavegame (Variables|SaveSet|GetLastDS_SaveSet))
  (SaveGame|SaveGametoSlot _bp_setsavegame (Variables|SaveSet|GetSetSlot)))

(event Custom|Event_AutoSaveGame
  (params (GameData :type DS%20HQ%20Save%20Game%20Structure) (SlotName :type String))
  ;[1 1 1] 自动存档游戏
  (Variables|SaveGame|SetNewGameData GameData)
  (bind _returnvalue (SaveGame|DoesSaveGameExist SlotName))
  (if _returnvalue
    (bind _returnvalue_2 (SaveGame|LoadGamefromSlot SlotName))
    (bind _asbp_fog_save_game (Utilities|Casting|CastToBP_FogSaveGame _returnvalue_2))
    (bind _output_get (Variables|保存游戏|SetBP_SaveGame _asbp_fog_save_game))
    (Variables|/Game/BP/SaveGame/BP_FogSaveGame.BP_FogSaveGame_C|SetDS_HQSaveGame _output_get (Variables|SaveGame|GetNewGameData))
    (else
      (bind _returnvalue_3 (SaveGame|CreateSaveGameObject "/Game/BP/SaveGame/BP_FogSaveGame.BP_FogSaveGame_C"))
      (bind _output_get_2 (Variables|保存游戏|SetBP_SaveGame _returnvalue_3))
      (Variables|/Game/BP/SaveGame/BP_FogSaveGame.BP_FogSaveGame_C|SetDS_HQSaveGame _output_get_2 (Variables|SaveGame|GetNewGameData))))
  (SaveGame|SaveGametoSlot (Variables|保存游戏|GetBP_SaveGame) SlotName)
  (Development|PrintString "保存成功"))

(event Custom|Event_BeginSaveGame
  ;[1 1 1] 初始化加载游戏
  (bind _returnvalue (SaveGame|DoesSaveGameExist "Auto"))
  (if _returnvalue
    (bind _returnvalue_2 (SaveGame|LoadGamefromSlot "Auto"))
    (bind _asbp_fog_save_game (Utilities|Casting|CastToBP_FogSaveGame _returnvalue_2))
    (bind _output_get (Variables|保存游戏|SetBP_SaveGame _asbp_fog_save_game))
    (Variables|保存游戏|SetLastSave%20Game (Variables|/Game/BP/SaveGame/BP_FogSaveGame.BP_FogSaveGame_C|GetDS_HQSaveGame _output_get))
    (else
      (bind _returnvalue_3 (SaveGame|CreateSaveGameObject "/Game/BP/SaveGame/BP_FogSaveGame.BP_FogSaveGame_C"))
      (bind _output_get_2 (Variables|保存游戏|SetBP_SaveGame _returnvalue_3))
      (Variables|保存游戏|SetLastSave%20Game (Variables|/Game/BP/SaveGame/BP_FogSaveGame.BP_FogSaveGame_C|GetDS_HQSaveGame _output_get_2)))))