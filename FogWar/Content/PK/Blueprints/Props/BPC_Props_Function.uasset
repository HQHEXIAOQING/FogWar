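; Blueprint component for prop effects on the player character, providing a health pickup effect and a temporary speed boost.
; BeginPlay caches player 0 as BP_PlayerClass, and both effect events act only while that character is not dead.
; The HP event writes the passed value directly into the player data's HP rather than adding it.
; The speed event overrides max walk speed, then restores a hardcoded default after a delay.
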(event Custom|Event_HPUp
  (params (AddHPValue :type Float%20%28double-precision%29))
  ;[1 1 1] 回血
  (if (not (Variables|/Game/BP/BP_FogChr/BP_Player/BP_PlayerClass.BP_PlayerClass_C|GetIsDie (Variables|Default|GetCharacter_Inst)))
    (Utilities|Struct|SetmembersinDS_PlayerData (Variables|/Game/BP/BP_FogChr/BP_Player/BP_PlayerClass.BP_PlayerClass_C|GetPlayerData (Variables|Default|GetCharacter_Inst)) AddHPValue)))

(event Custom|Event_speedUP
  (params (SpeedUpDuration :type Float%20%28single-precision%29) (最大行走速度 :type Float%20%28single-precision%29))
  ;[1 1 1] 加速
  (if (not (Variables|/Game/BP/BP_FogChr/BP_Player/BP_PlayerClass.BP_PlayerClass_C|GetIsDie (Variables|Default|GetCharacter_Inst)))
    (Variables|/Script/Engine.CharacterMovementComponent|SetMaxWalkSpeed (Variables|/Script/Engine.Character|GetCharacterMovement (Variables|Default|GetCharacter_Inst)) 最大行走速度)
    (Utilities|FlowControl|Delay SpeedUpDuration)
    (Variables|/Script/Engine.CharacterMovementComponent|SetMaxWalkSpeed (Variables|/Script/Engine.Character|GetCharacterMovement (Variables|Default|GetCharacter_Inst)) 6e+02)))

(event EventBeginPlay
  ;[1 1 1] 初始获得玩家实例
  (bind _asbp_player_class (Utilities|Casting|CastToBP_PlayerClass (Game|GetPlayerCharacter 0)))
  (Variables|Default|SetCharacter_Inst _asbp_player_class))